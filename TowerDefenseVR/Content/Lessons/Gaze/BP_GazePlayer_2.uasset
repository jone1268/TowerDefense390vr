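; VR gaze player that lets the user hover over and select actors by looking at them.
; Each tick it moves the spring arm to the camera and line-traces forward, sending hover on/off messages as the target changes.
; Targets confirming ProgressMessage build frame-based dwell progress, receiving SelectMessage every tick once full; otherwise progress resets.
; That progress drives a dynamic billboard material as the reticle.
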(event EventTick
  (params (DeltaSeconds :type Float%20%28single-precision%29))
  (Utilities|FlowControl|Sequence
    (:then_0
      (CallFunction|UpdateSpringArm))
    (:then_1
      (bind (_location _forward_vector) (CallFunction|GetPlayerVRCameraProperties))
      (bind _outhit (Collision|LineTraceByChannel _location (+ _location (* _forward_vector 1e+04)) "TraceTypeQuery1" false 0 "None"))
      (Utilities|FlowControl|Sequence
        (:then_0
          (if (== (Variables|Default|GetLastTraceActor) (.HitActor (Collision|BreakHitResult _outhit)))
            (bind _selectable (Class|BPIGazeInteraction|Progress(Message) (.HitActor (Collision|BreakHitResult _outhit))))
            (if _selectable
              (bind _output_get (Variables|Default|SetHoverProgress (+ (Variables|Default|GetHoverProgress) 0.02)))
              (if (>= _output_get 1.0)
                (Class|BPIGazeInteraction|Select(Message) (.HitActor (Collision|BreakHitResult _outhit))))
              (else
                (Variables|Default|SetHoverProgress 0.0 :!label _label)))
            (else
              (Class|BPIGazeInteraction|Hoveron(Message) (.HitActor (Collision|BreakHitResult _outhit)))
              (Class|BPIGazeInteraction|HoverOff(Message) (Variables|Default|GetLastTraceActor))
              (goto _label))))
        (:then_1
          (Variables|Default|SetLastTraceActor (.HitActor (Collision|BreakHitResult _outhit)))
          (Rendering|Material|SetScalarParameterValue (Variables|Default|GetReticleDMI) "progress" (Variables|Default|GetHoverProgress) :!class /Script/Engine.MaterialInstanceDynamic))))))

(fn ConstructionScript
  (bind _dynamic_material (CallFunction|CreateDynamicBillboardMaterial (Variables|Default|GetMaterialBillboard)))
  (Variables|Default|SetReticleDMI _dynamic_material))

(fn UpdateSpringArm
  (bind _location (CallFunction|GetPlayerVRCameraProperties))
  (Transformation|SetWorldLocation (Variables|Default|GetSpringArm) _location false false)
  (return))