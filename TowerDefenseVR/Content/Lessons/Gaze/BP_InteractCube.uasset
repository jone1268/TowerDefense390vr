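; Gaze-lesson interactable cube that changes color on hover and shakes when selected.
; The construction script creates a dynamic material, and the hover events swap its two checker colors.
; Select plays the Movement timeline, scaling fresh random location and rotation offsets each update, and clears Selectable until it finishes.
; Progress returns Selectable; a line-color cycle timeline exists but is never triggered.
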(event EventBeginPlay)

(event Collision|EventActorBeginOverlap
  (params (OtherActor :type Actor%20Object%20Reference)))

(event EventHoveron
  (bind _dmi (Variables|Default|GetDMI))
  (Rendering|Material|SetVectorParameterValue _dmi "CheckColor1" "(R=0.940654,G=0.814732,B=0.000000,A=1.000000)" :!class /Script/Engine.MaterialInstanceDynamic)
  (Rendering|Material|SetVectorParameterValue _dmi "CheckerColor2" "(R=0.003040,G=0.940654,B=0.000000,A=1.000000)" :!class /Script/Engine.MaterialInstanceDynamic))

(event EventTick
  (params (DeltaSeconds :type Float%20%28single-precision%29)))

(event EventHoverOff
  (bind _dmi (Variables|Default|GetDMI))
  (Rendering|Material|SetVectorParameterValue _dmi "CheckColor1" "(R=0.597202,G=0.056128,B=0.056128,A=1.000000)" :!class /Script/Engine.MaterialInstanceDynamic)
  (Rendering|Material|SetVectorParameterValue _dmi "CheckerColor2" "(R=0.099899,G=0.000000,B=0.068478,A=1.000000)" :!class /Script/Engine.MaterialInstanceDynamic))

(event EventSelect
  (bind _cube (Variables|Default|GetCube))
  (Variables|Default|SetSelectable false)
  (bind _data (Timeline|Movement PlayFromStart)
    (:Update
      (Transformation|SetRelativeLocation _cube (* (Math|Vector|MakeVector (Math|Random|RandomFloatinRange -2e+01 2e+01) (Math|Random|RandomFloatinRange -2e+01 2e+01) (Math|Random|RandomFloatinRange -2e+01 2e+01)) _data) true false)
      (Transformation|SetRelativeRotation _cube (Math|Rotator|MakeRotator (* _data (Math|Random|RandomFloatinRange -2e+01 2e+01)) (* _data (Math|Random|RandomFloatinRange -2e+01 2e+01)) (* _data (Math|Random|RandomFloatinRange -2e+01 2e+01))) false false))
    (:Finished
      (Variables|Default|SetSelectable true))))

(fn ConstructionScript
  (bind _returnvalue (Rendering|Material|CreateDynamicMaterialInstance (Variables|Default|GetCube) 0 0 :!class /Script/Engine.PrimitiveComponent))
  (Variables|Default|SetDMI _returnvalue))

(fn Progress
  (return (Variables|Default|GetSelectable)))