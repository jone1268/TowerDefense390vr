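; BP_Button is a button for the Gaze lesson, with hover and select events that give visual feedback.
; The construction script creates a dynamic material, which the hover events recolor between cyan and red.
; Select plays a timeline that offsets the mesh downward, disabling Selectable until it finishes and then setting Pressed.
; The Progress function returns Selectable, exposing whether the button can currently be selected.
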(event EventHoverOff
  (Rendering|Material|SetVectorParameterValue (Variables|Default|GetDMI) "Color" "(R=0.919454,G=0.000000,B=0.049146,A=1.000000)" :!class /Script/Engine.MaterialInstanceDynamic))

(event EventSelect
  (Variables|Default|SetSelectable false)
  (bind _data (Timeline|Selected PlayFromStart)
    (:Update
      (Transformation|SetRelativeLocation (Variables|Default|GetStaticMesh) (* "0, 0,-30.000000" _data) false false))
    (:Finished
      (Variables|Default|SetSelectable true)
      (Variables|Default|SetPressed true))))

(event EventHoveron
  (Rendering|Material|SetVectorParameterValue (Variables|Default|GetDMI) "Color" "(R=0.077343,G=0.940654,B=0.888974,A=1.000000)" :!class /Script/Engine.MaterialInstanceDynamic))

(fn ConstructionScript
  (bind _returnvalue (Rendering|Material|CreateDynamicMaterialInstance (Variables|Default|GetStaticMesh) 0 0 :!class /Script/Engine.PrimitiveComponent))
  (Variables|Default|SetDMI _returnvalue))

(fn Progress
  (return (Variables|Default|GetSelectable)))