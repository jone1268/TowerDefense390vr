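; A gaze-lesson cube actor that changes its checker colors on hover and explodes when selected.
; The construction script creates a dynamic material on the cube, which the hover events recolor.
; Select clears the Selectable flag reported by Progress, spawns an explosion emitter and destroys the actor.
; A line-color timeline is present but never runs.
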(event EventBeginPlay)

(event Collision|EventActorBeginOverlap
  (params (OtherActor :type Actor%20Object%20Reference)))

(event EventHoveron
  (bind _dmi (Variables|Default|GetDMI))
  (Rendering|Material|SetVectorParameterValue _dmi "CheckColor1" "(R=0.161895,G=0.183042,B=0.940654,A=1.000000)" :!class /Script/Engine.MaterialInstanceDynamic)
  (Rendering|Material|SetVectorParameterValue _dmi "CheckerColor2" "(R=0.174113,G=0.033874,B=0.153991,A=1.000000)" :!class /Script/Engine.MaterialInstanceDynamic))

(event EventTick
  (params (DeltaSeconds :type Float%20%28single-precision%29)))

(event EventHoverOff
  (bind _dmi (Variables|Default|GetDMI))
  (Rendering|Material|SetVectorParameterValue _dmi "CheckColor1" "(R=0.102783,G=0.827515,B=0.629475,A=1.000000)" :!class /Script/Engine.MaterialInstanceDynamic)
  (Rendering|Material|SetVectorParameterValue _dmi "CheckerColor2" "(R=0.742984,G=0.776103,B=0.756059,A=1.000000)" :!class /Script/Engine.MaterialInstanceDynamic))

(event EventSelect
  (Variables|Default|SetSelectable false)
  (Effects|SpawnEmitteratLocation "/Game/Effects/Particles/Explosion/P_AsteroidExplosion.P_AsteroidExplosion" (Transformation|GetWorldLocation (Variables|Default|GetCube)))
  (Actor|DestroyActor))

(fn ConstructionScript
  (bind _returnvalue (Rendering|Material|CreateDynamicMaterialInstance (Variables|Default|GetCube) 0 0 :!class /Script/Engine.PrimitiveComponent))
  (Variables|Default|SetDMI _returnvalue))

(fn Progress
  (return (Variables|Default|GetSelectable)))