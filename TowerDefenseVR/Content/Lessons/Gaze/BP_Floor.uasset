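; Gaze lesson floor actor that slides opposite the VR camera's horizontal forward vector, suggesting travel in the gaze direction.
; Tick applies the offset scaled by delta time and checks the floor's distance against a large camera-relative threshold.
; Past it, the FadeColors timeline tints the construction-script dynamic material, then the floor resets position and checker colors.
; A ColorCycle timeline for line color exists but never runs.
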(event EventBeginPlay)

(event Collision|EventActorBeginOverlap
  (params (OtherActor :type Actor%20Object%20Reference)))

(event EventTick
  (params (DeltaSeconds :type Float%20%28single-precision%29))
  (bind _returnvalue (Utilities|Time|GetWorldDeltaSeconds))
  (bind _floor (Variables|Default|GetFloor))
  (bind _dmi (Variables|Default|GetDMI))
  (bind _dmi_2 (Variables|Default|GetDMI))
  (bind _returnvalue_2 (Transformation|GetWorldLocation _floor))
  (bind _returnvalue_3 (* _returnvalue -1e+02))
  (bind (_location _forward_vector) (CallFunction|GetPlayerVRCameraProperties))
  (Transformation|AddActorWorldOffset (Math|Vector|MakeVector (* _returnvalue_3 (.X (Math|Vector|BreakVector _forward_vector))) (* _returnvalue_3 (.Y (Math|Vector|BreakVector _forward_vector))) 0.0))
  (if (or (>= (Math|Float|Absolute(Float) (.x _returnvalue_2)) (Math|Float|Absolute(Float) (+ (.x _location) 1e+05))) (>= (Math|Float|Absolute(Float) (.y _returnvalue_2)) (Math|Float|Absolute(Float) (+ (.y _location) 1e+05))))
    (bind _color (Timeline|FadeColors Play)
      (:Update
        (Rendering|Material|SetVectorParameterValue _dmi "CheckColor1" _color :!class /Script/Engine.MaterialInstanceDynamic)
        (Rendering|Material|SetVectorParameterValue _dmi "CheckerColor2" _color :!class /Script/Engine.MaterialInstanceDynamic)
        (Rendering|Material|SetVectorParameterValue _dmi "LineColor" _color :!class /Script/Engine.MaterialInstanceDynamic))
      (:Finished
        (Transformation|SetActorLocation (Math|Vector|MakeVector 0.0 0.0 0.0) false false)
        (Rendering|Material|SetVectorParameterValue _dmi_2 "CheckColor1" "(R=0.001214,G=0.001518,B=0.006512,A=1.000000)" :!class /Script/Engine.MaterialInstanceDynamic)
        (Rendering|Material|SetVectorParameterValue _dmi_2 "CheckerColor2" "(R=0.001214,G=0.001518,B=0.006512,A=1.000000)" :!class /Script/Engine.MaterialInstanceDynamic)
        (Timeline|FadeColors SetNewTime)))))

(fn ConstructionScript
  (bind _returnvalue (Rendering|Material|CreateDynamicMaterialInstance (Variables|Default|GetFloor) 0 0 :!class /Script/Engine.PrimitiveComponent))
  (Variables|Default|SetDMI _returnvalue))