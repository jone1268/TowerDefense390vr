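; An interactable cube for a gaze lesson that reacts to hover and selection.
; The construction script creates a dynamic material on the cube, and Hoveron and HoverOff swap its checker color parameters.
; Select plays a Scale timeline that resizes the cube, clearing Selectable until it finishes; the Progress function reports that flag.
; A ColorCycle timeline meant to drive the line color is never triggered.
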(event EventBeginPlay)

(event Collision|EventActorBeginOverlap
  (params (OtherActor :type Actor%20Object%20Reference)))

(event EventHoveron
  (bind _dmi (Variables|Default|GetDMI))
  (Rendering|Material|SetVectorParameterValue _dmi "CheckColor1" "(R=0.005212,G=0.947307,B=0.733843,A=1.000000)" :!class /Script/Engine.MaterialInstanceDynamic)
  (Rendering|Material|SetVectorParameterValue _dmi "CheckerColor2" "(R=0.940654,G=0.042195,B=0.077256,A=1.000000)" :!class /Script/Engine.MaterialInstanceDynamic))

(event EventTick
  (params (DeltaSeconds :type Float%20%28single-precision%29)))

(event EventHoverOff
  (bind _dmi (Variables|Default|GetDMI))
  (Rendering|Material|SetVectorParameterValue _dmi "CheckColor1" "(R=0.173230,G=0.208438,B=0.597202,A=1.000000)" :!class /Script/Engine.MaterialInstanceDynamic)
  (Rendering|Material|SetVectorParameterValue _dmi "CheckerColor2" "(R=0.094855,G=0.099899,B=0.008329,A=1.000000)" :!class /Script/Engine.MaterialInstanceDynamic))

(event EventSelect
  (Variables|Default|SetSelectable false)
  (bind _data (Timeline|Scale PlayFromStart)
    (:Update
      (Transformation|SetRelativeScale3D (Variables|Default|GetCube) (Math|Vector|MakeVector _data _data _data)))
    (:Finished
      (Variables|Default|SetSelectable true))))

(fn ConstructionScript
  (bind _returnvalue (Rendering|Material|CreateDynamicMaterialInstance (Variables|Default|GetCube) 0 0 :!class /Script/Engine.PrimitiveComponent))
  (Variables|Default|SetDMI _returnvalue))

(fn Progress
  (return (Variables|Default|GetSelectable)))