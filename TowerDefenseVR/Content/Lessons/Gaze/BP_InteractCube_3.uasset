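; BP_InteractCube_3 is a gaze-lesson cube that reacts to hover and select events.
; Construction creates a dynamic material instance, whose two checker colors switch between bright cyan/green on hover and gray off hover.
; Select locks selection, exposed through Progress, while the Scale timeline plays, but its relative-move delta is zero, so the cube stays put.
; The LineColor cycle timeline is never triggered, and the VR camera lookup goes unused.
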(event EventBeginPlay)

(event Collision|EventActorBeginOverlap
  (params (OtherActor :type Actor%20Object%20Reference)))

(event EventHoveron
  (bind _dmi (Variables|Default|GetDMI))
  (Rendering|Material|SetVectorParameterValue _dmi "CheckColor1" "(R=0.000000,G=0.947307,B=0.896261,A=1.000000)" :!class /Script/Engine.MaterialInstanceDynamic)
  (Rendering|Material|SetVectorParameterValue _dmi "CheckerColor2" "(R=0.000000,G=0.940654,B=0.055724,A=1.000000)" :!class /Script/Engine.MaterialInstanceDynamic))

(event EventTick
  (params (DeltaSeconds :type Float%20%28single-precision%29)))

(event EventHoverOff
  (bind _dmi (Variables|Default|GetDMI))
  (Rendering|Material|SetVectorParameterValue _dmi "CheckColor1" "(R=0.573412,G=0.597202,B=0.597179,A=1.000000)" :!class /Script/Engine.MaterialInstanceDynamic)
  (Rendering|Material|SetVectorParameterValue _dmi "CheckerColor2" "(R=0.616048,G=0.616048,B=0.616048,A=1.000000)" :!class /Script/Engine.MaterialInstanceDynamic))

(event EventSelect
  (Variables|Default|SetSelectable false)
  (bind _data (Timeline|Scale PlayFromStart)
    (:Update
      (bind _forward_vector (CallFunction|GetPlayerVRCameraProperties))
      (Transformation|AddRelativeLocation (Variables|Default|GetCube) (* "0, 0, 0" _data) true false))
    (:Finished
      (Variables|Default|SetSelectable true))))

(fn ConstructionScript
  (bind _returnvalue (Rendering|Material|CreateDynamicMaterialInstance (Variables|Default|GetCube) 0 0 :!class /Script/Engine.PrimitiveComponent))
  (Variables|Default|SetDMI _returnvalue))

(fn Progress
  (return (Variables|Default|GetSelectable)))