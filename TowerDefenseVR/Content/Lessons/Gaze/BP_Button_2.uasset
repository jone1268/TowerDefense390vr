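; BP_Button_2 is a gaze-lesson button whose mesh changes color through a dynamic material instance created in the construction script.
; Hoveron shows an inverted color computed from ColorNegate minus Color, and HoverOff restores Color.
; Select applies the current Color, then randomizes the stored value, which appears on later hover changes.
; Selection also clears Selectable for a short delay, and Progress returns that flag.
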(event EventHoverOff
  (Rendering|Material|SetVectorParameterValue (Variables|Default|GetDMI) "Color" (Variables|Default|GetColor) :!class /Script/Engine.MaterialInstanceDynamic))

(event EventSelect
  (Variables|Default|SetSelectable false)
  (Rendering|Material|SetVectorParameterValue (Variables|Default|GetDMI) "Color" (Variables|Default|GetColor) :!class /Script/Engine.MaterialInstanceDynamic)
  (Variables|Default|SetColor (Utilities|Struct|MakeLinearColor (Math|Random|RandomFloatinRange 0.0 1.0) (Math|Random|RandomFloatinRange 0.0 1.0) (Math|Random|RandomFloatinRange 0.0 1.0) 1.0))
  (Utilities|FlowControl|Delay 2.5)
  (Variables|Default|SetSelectable true))

(event EventHoveron
  (bind _color (Variables|Default|GetColor))
  (bind _color_negate (Variables|Default|GetColor_negate))
  (bind (_r _g _b) (Utilities|Struct|BreakLinearColor _color_negate))
  (bind (_r_2 _g_2 _b_2 _a) (Utilities|Struct|BreakLinearColor _color))
  (Rendering|Material|SetVectorParameterValue (Variables|Default|GetDMI) "Color" (Utilities|Struct|MakeLinearColor (- _r _r_2) (- _g _g_2) (- _b _b_2) _a) :!class /Script/Engine.MaterialInstanceDynamic))

(fn ConstructionScript
  (bind _returnvalue (Rendering|Material|CreateDynamicMaterialInstance (Variables|Default|GetStaticMesh) 0 0 :!class /Script/Engine.PrimitiveComponent))
  (Variables|Default|SetDMI _returnvalue))

(fn Progress
  (return (Variables|Default|GetSelectable)))