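; Gaze-lesson cube actor that highlights on hover and explodes when selected.
; The construction script creates a dynamic material instance on the cube, and the hover events switch its checker colors between yellows and red/black.
; Select clears Selectable, which the Progress function reports, then spawns an asteroid explosion and destroys the actor.
; A ColorCycle timeline for line color is present but never runs.
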(event EventBeginPlay)

(event Collision|EventActorBeginOverlap
  (params (OtherActor :type Actor%20Object%20Reference)))

(event EventHoveron
  (bind _dmi (Variables|Default|GetDMI))
  (Rendering|Material|SetVectorParameterValue _dmi "CheckColor1" "(R=0.940654,G=0.844392,B=0.000000,A=1.000000)" :!class /Script/Engine.MaterialInstanceDynamic)
  (Rendering|Material|SetVectorParameterValue _dmi "CheckerColor2" "(R=1.000000,G=0.962660,B=0.000000,A=1.000000)" :!class /Script/Engine.MaterialInstanceDynamic))

(event EventTick
  (params (DeltaSeconds :type Float%20%28single-precision%29)))

(event EventHoverOff
  (bind _dmi (Variables|Default|GetDMI))
  (Rendering|Material|SetVectorParameterValue _dmi "CheckColor1" "(R=0.827515,G=0.000000,B=0.024029,A=1.000000)" :!class /Script/Engine.MaterialInstanceDynamic)
  (Rendering|Material|SetVectorParameterValue _dmi "CheckerColor2" "(R=0.000000,G=0.000000,B=0.000000,A=1.000000)" :!class /Script/Engine.MaterialInstanceDynamic))

(event EventSelect
  (Variables|Default|SetSelectable false)
  (Effects|SpawnEmitteratLocation "/Game/Effects/Particles/Explosion/P_AsteroidExplosion.P_AsteroidExplosion" (Transformation|GetWorldLocation (Variables|Default|GetCube)))
  (Actor|DestroyActor))

(fn ConstructionScript
  (bind _returnvalue (Rendering|Material|CreateDynamicMaterialInstance (Variables|Default|GetCube) 0 0 :!class /Script/Engine.PrimitiveComponent))
  (Variables|Default|SetDMI _returnvalue))

(fn Progress
  (return (Variables|Default|GetSelectable)))