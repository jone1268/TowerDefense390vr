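; BP_BlastingBox is a physics-lesson trigger box that fires once when a Character overlaps it.
; On that overlap a timeline with an ease-in expo curve lowers StaticMesh1 along Z from its starting relative location, like a plunger being pressed.
; It also sends PhysicsInteractMessage to every actor in the InteractWith array, so linked objects can react.
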(event OnComponentBeginOverlap(Box)
  (params (OtherActor :type Actor%20Object%20Reference) (OtherComp :type Primitive%20Component%20Object%20Reference) (OtherBodyIndex :type Integer) (bFromSweep :type Boolean) (SweepResult :type Hit%20Result%20Structure%20%28by%20ref%29))
  (if (not (Variables|Default|GetOverlapFired))
    (Utilities|Casting|CastToCharacter OtherActor)
    (Utilities|FlowControl|Sequence
      (:then_0
        (Variables|Default|SetOverlapFired true))
      (:then_1
        (Variables|Default|SetArmLocation (Variables|/Script/Engine.SceneComponent|GetRelativeLocation (Variables|Default|GetStaticMesh1))))
      (:then_2
        (bind _curve_easeinexpo (Timeline|Timeline_0 PlayFromStart)
          (:Update
            (Transformation|SetRelativeLocation (Variables|Default|GetStaticMesh1) (+ (Variables|Default|GetArmLocation) (Math|Vector|MakeVector 0.0 0.0 (* _curve_easeinexpo -15.0))) false false))))
      (:then_3
        (for _array_element (Variables|Default|GetInteractWith)
          (Class|BPIPhysicsInteract|PhysicsInteract(Message) _array_element))))))

(fn ConstructionScript)